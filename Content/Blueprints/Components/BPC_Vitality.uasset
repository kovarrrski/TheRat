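; Vitality component that tracks health and a defeated state, presumably for the actor that owns it.
; Current health starts at the maximum on BeginPlay.
; ReceiveDamage subtracts damage, clamps health between zero and the maximum, and sets the defeated flag at zero.
; Once defeated, further damage is ignored, and no event is broadcast on damage or defeat.
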(event EventBeginPlay
  (Variables|Default|SetCurentHeath (Variables|Default|GetMaxHealth%20)))

(event EventTick
  (params (DeltaSeconds :type Float%20%28single-precision%29)))

(fn ReceiveDamage
  (params (Damage :type Float%20%28double-precision%29))
  (if (not (Variables|Default|GetIsDefetead))
    ;[1 1 1] - Damage (1)
    (Variables|Default|SetCurentHeath (Math|Float|Clamp(Float) (- (Variables|Default|GetCurentHeath) Damage) 0.0 (Variables|Default|GetMaxHealth%20)))
    ;[1 1 1] Check and Set Defeated State
    (if (<= (Variables|Default|GetCurentHeath) 0.0)
      (Variables|Default|SetIsDefetead true))))